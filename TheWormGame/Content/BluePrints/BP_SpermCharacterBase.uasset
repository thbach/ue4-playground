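; BP_SpermCharacterBase is a sperm character base Blueprint that animates a procedural wobble on its SpermHead component.
; BeginPlay picks a random Seed that sets the wobble frequency, so instances can oscillate at different rates.
; Each Tick sets the head's relative roll from a sine of time since creation, keeping pitch upright at a fixed angle.
; The roll amplitude is SinAngleMult scaled by DeltaSeconds, so it varies with frame rate.
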(event `self.ReceiveBeginPlay`
  (set `self.Seed` (+ (* (`KismetMathLibrary.RandomFloat`) 10.0) 10.0)))

(event `self.ReceiveTick`
  (params (DeltaSeconds :type "Float (single-precision)"))
  (`SceneComponent.K2_SetRelativeRotation` (`self.SpermHead`) (`KismetMathLibrary.MakeRotator` (* (* DeltaSeconds (`self.SinAngleMult`)) (`KismetMathLibrary.Sin` (* (`self.GetGameTimeSinceCreation`) (`self.Seed`)))) 90.0) false true))

(fn `UserConstructionScript`)