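; BP_SpawnPoolAI is an actor, named as an AI spawn pool, that follows the player along the X axis.
; Each Tick it sets Respawn by testing whether the player pawn's X is at or below XMaxBounds.
; While Respawn is true, it moves to the player's X plus XOffset, keeping its own Y and Z.
; The graph itself contains no spawning or pooling logic.
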(event `self.ReceiveTick`
  (params (DeltaSeconds :type "Float (single-precision)"))
  (bind (_returnvalue_x _returnvalue_y _returnvalue_z) (`KismetMathLibrary.BreakVector` (`self.K2_GetActorLocation`)))
  (bind _returnvalue_x_2 (`KismetMathLibrary.BreakVector` (`self.K2_GetActorLocation` (`GameplayStatics.GetPlayerPawn` 0))))
  (`parent.ReceiveTick` DeltaSeconds)
  (bind _output_get (set `self.bRespawn` (<= _returnvalue_x_2 (`self.XMaxBounds`))))
  (if _output_get
    (`self.K2_SetActorLocation` (`KismetMathLibrary.MakeVector` (+ _returnvalue_x_2 (`self.XOffset`)) _returnvalue_y _returnvalue_z))))

(fn `UserConstructionScript`
  (`parent.UserConstructionScript`))