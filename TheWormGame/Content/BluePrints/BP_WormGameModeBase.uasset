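; Game mode for the worm game that drives the start and game-over screens.
; On BeginPlay it adds the health bar HUD and briefly shows a start widget before removing it.
; The GameOver event picks a win, timeout or lose widget from its flags, waits a restart delay, then reloads the main level.
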(event `self.ReceiveBeginPlay`
  (bind _returnvalue (`|CreateWidget` "/Game/BluePrints/UI/WBP_HealthBar.WBP_HealthBar_C"))
  (`UserWidget.AddToViewport` _returnvalue 0)
  (bind _returnvalue_2 (`|CreateWidget` "/Game/BluePrints/UI/WBP_GameStart.WBP_GameStart_C"))
  (`UserWidget.AddToViewport` _returnvalue_2 0)
  (`KismetSystemLibrary.Delay` 2.0)
  (`Widget.RemoveFromParent` _returnvalue_2))

(event `self.GameOver`
  (params (PlayerWon :type Boolean) (bIsTimeout :type Boolean))
  (if PlayerWon
    (bind _returnvalue (`|CreateWidget` "/Game/BluePrints/UI/WBP_GameOverWin.WBP_GameOverWin_C"))
    (`UserWidget.AddToViewport` _returnvalue 0)
    (elif bIsTimeout
      (bind _returnvalue_2 (`|CreateWidget` "/Game/BluePrints/UI/WBP_GameOverTimeOut.WBP_GameOverTimeOut_C"))
      (`UserWidget.AddToViewport` _returnvalue_2 0)
      (else
        (bind _returnvalue_3 (`|CreateWidget` "/Game/BluePrints/UI/WBP_GameOverLose.WBP_GameOverLose_C"))
        (`UserWidget.AddToViewport` _returnvalue_3 0))))
  (`KismetSystemLibrary.Delay` (`self.RestartDelay`))
  (`GameplayStatics.OpenLevel` (`self.MainLevel`)))

(fn `UserConstructionScript`)